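; VR player controller that handles locomotion, turning and two-handed grabbing for BP_VRCharacter.
; BeginPlay adds the VR input mapping context; movement follows the headset camera's yaw and turning adjusts control yaw scaled by frame time.
; Each grab press sphere-overlaps around that motion controller and sends Grab to the first IGrabbable found, storing it per hand until release sends Release and clears it.
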(event `self.ReceiveBeginPlay`
  (`EnhancedInputSubsystemInterface.AddMappingContext` (pcsubsystem `EnhancedInputLocalPlayerSubsystem` self) "/Game/Blueprints/Input/IMC_VRPlayer.IMC_VRPlayer" 1 (struct)))

(event `EnhancedInput|/Game/Blueprints/Input/IA_VR_Move`
  (params (ActionValue :type "Vector2D Structure") (ElapsedSeconds :type "Float (double-precision)") (TriggeredSeconds :type "Float (double-precision)") (InputAction :type "InputAction Object Reference" :default "/Game/Blueprints/Input/IA_VR_Move.IA_VR_Move"))
  (bind (_x _y) (`KismetMathLibrary.BreakVector2D` ActionValue))
  (:`Triggered`
    (bind _asbp_vrcharacter (cast `/Game/Blueprints/BP_VRCharacter` (`self.K2_GetPawn`)))
    (bind _returnvalue (`KismetMathLibrary.MakeRotator` 0.0 0.0 (.yaw (`SceneComponent.K2_GetComponentRotation` (`/Game/Blueprints/BP_VRCharacter.Camera` _asbp_vrcharacter)))))
    (`Pawn.AddMovementInput` _asbp_vrcharacter (`KismetMathLibrary.GetForwardVector` _returnvalue) _y false)
    (`Pawn.AddMovementInput` _asbp_vrcharacter (`KismetMathLibrary.GetRightVector` _returnvalue) _x false)))

(event `EnhancedInput|/Game/Blueprints/Input/IA_VR_Turn`
  (params (ActionValue :type "Float (double-precision)") (ElapsedSeconds :type "Float (double-precision)") (TriggeredSeconds :type "Float (double-precision)") (InputAction :type "InputAction Object Reference" :default "/Game/Blueprints/Input/IA_VR_Turn.IA_VR_Turn"))
  (:`Triggered`
    (`self.SetControlRotation` (`KismetMathLibrary.MakeRotator` 0.0 0.0 (+ (.yaw (`self.GetControlRotation`)) (* (* ActionValue (`self.TurnSpeed`)) (`GameplayStatics.GetWorldDeltaSeconds`)))))))

(event `EnhancedInput|/Game/Blueprints/Input/IA_VR_Grab_Left`
  (params (ActionValue :type Boolean) (ElapsedSeconds :type "Float (double-precision)") (TriggeredSeconds :type "Float (double-precision)") (InputAction :type "InputAction Object Reference" :default "/Game/Blueprints/Input/IA_VR_Grab_Left.IA_VR_Grab_Left"))
  (bind _returnvalue (`self.K2_GetPawn`))
  (bind _heldactorleft (`self.HeldActorLeft`))
  (:`Started`
    (bind _asbp_vrcharacter (cast `/Game/Blueprints/BP_VRCharacter` _returnvalue))
    (bind _grabbedactor (`self.TryGrab` (`/Game/Blueprints/BP_VRCharacter.MotionControllerLeft` _asbp_vrcharacter)))
    (set `self.HeldActorLeft` _grabbedactor))
  (:`Completed`
    (bind _asbp_vrcharacter_2 (cast `/Game/Blueprints/BP_VRCharacter` _returnvalue))
    (if (`KismetSystemLibrary.IsValid` _heldactorleft)
      (message `/Game/Blueprints/IGrabbable.Release` _heldactorleft (`/Game/Blueprints/BP_VRCharacter.MotionControllerLeft` _asbp_vrcharacter_2))
      (set `self.HeldActorLeft` null))))

(event `EnhancedInput|/Game/Blueprints/Input/IA_VR_Grab_Right`
  (params (ActionValue :type Boolean) (ElapsedSeconds :type "Float (double-precision)") (TriggeredSeconds :type "Float (double-precision)") (InputAction :type "InputAction Object Reference" :default "/Game/Blueprints/Input/IA_VR_Grab_Right.IA_VR_Grab_Right"))
  (bind _returnvalue (`self.K2_GetPawn`))
  (bind _heldactorright (`self.HeldActorRight`))
  (:`Started`
    (bind _asbp_vrcharacter (cast `/Game/Blueprints/BP_VRCharacter` _returnvalue))
    (bind _grabbedactor (`self.TryGrab` (`/Game/Blueprints/BP_VRCharacter.MotionControllerRight` _asbp_vrcharacter)))
    (set `self.HeldActorRight` _grabbedactor))
  (:`Completed`
    (bind _asbp_vrcharacter_2 (cast `/Game/Blueprints/BP_VRCharacter` _returnvalue))
    (if (`KismetSystemLibrary.IsValid` _heldactorright)
      (message `/Game/Blueprints/IGrabbable.Release` _heldactorright (`/Game/Blueprints/BP_VRCharacter.MotionControllerRight` _asbp_vrcharacter_2))
      (set `self.HeldActorRight` null))))

(fn `TryGrab`
  (params (MotionController :type "MotionControllerComponent Object Reference"))
  (returns (GrabbedActor :type "Actor Object Reference"))
  (bind _outactors (`KismetSystemLibrary.SphereOverlapActors` (`SceneComponent.K2_GetComponentLocation` MotionController) (`self.GrabRadius`) (`|MakeArray` "ObjectTypeQuery2" "ObjectTypeQuery4" :!type "EObjectTypeQuery Enum") null (`|MakeArray` (`self.K2_GetPawn`))))
  (for _array_element _outactors
    (if (`KismetSystemLibrary.DoesImplementInterface` _array_element "/Game/Blueprints/IGrabbable.IGrabbable_C")
      (message `/Game/Blueprints/IGrabbable.Grab` _array_element MotionController)
      (return _array_element)))
  (return null))

(fn `UserConstructionScript`)