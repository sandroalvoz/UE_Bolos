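; Bowling ball actor that a motion controller can grab, carry and throw, with a reset to its starting transform.
; Grab disables physics on the Sphere and attaches it to the controller.
; While held, Tick blends frame-to-frame movement into a smoothed throw velocity, which Release applies, scaled by ThrowStrength, after re-enabling physics.
; ResetBall detaches the ball, teleports it to the transform saved at BeginPlay and zeroes its linear and angular velocity.
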(event `self.ReceiveBeginPlay`
  (bind _returnvalue (`SceneComponent.K2_GetComponentToWorld` (`self.Sphere`)))
  (set `self.StartTransform` _returnvalue)
  (set `self.LastHeldLocation` (.location _returnvalue)))

(event `self.ReceiveTick`
  (params (DeltaSeconds :type "Float (single-precision)"))
  (bind _returnvalue (`SceneComponent.K2_GetComponentLocation` (`self.Sphere`)))
  (if (and (`self.bIsHeld`) (> DeltaSeconds 0.0))
    (set `self.ThrowVelocity` (`KismetMathLibrary.VLerp` (`self.ThrowVelocity`) (/ (- _returnvalue (`self.LastHeldLocation`)) DeltaSeconds) 0.5))
    (set `self.LastHeldLocation` _returnvalue)))

(event `/Game/Blueprints/IGrabbable.Grab`
  (params (MotionController :type "MotionControllerComponent Object Reference"))
  (bind _sphere (`self.Sphere`))
  (`PrimitiveComponent.SetSimulatePhysics` _sphere false)
  (`SceneComponent.K2_AttachToComponent` _sphere MotionController "None" "KeepWorld" "KeepWorld" "KeepWorld" false)
  (set `self.LastHeldLocation` (`SceneComponent.K2_GetComponentLocation` _sphere))
  (set `self.ThrowVelocity` (`KismetMathLibrary.MakeVector` 0.0))
  (set `self.bIsHeld` true))

(event `/Game/Blueprints/IGrabbable.Release`
  (params (MotionController :type "MotionControllerComponent Object Reference"))
  (bind _sphere (`self.Sphere`))
  (`SceneComponent.K2_DetachFromComponent` _sphere "KeepWorld" "KeepWorld" "KeepWorld" true)
  (set `self.bIsHeld` false)
  (`PrimitiveComponent.SetSimulatePhysics` _sphere true)
  (`PrimitiveComponent.SetPhysicsLinearVelocity` _sphere (* (`self.ThrowVelocity`) (`self.ThrowStrength`)) false "None"))

(fn `ResetBall`
  (bind _sphere (`self.Sphere`))
  (`PrimitiveComponent.SetSimulatePhysics` _sphere false)
  (`SceneComponent.K2_DetachFromComponent` _sphere "KeepWorld" "KeepWorld" "KeepWorld" true)
  (set `self.bIsHeld` false)
  (`SceneComponent.K2_SetWorldTransform` _sphere (`self.StartTransform`) false true)
  (`PrimitiveComponent.SetSimulatePhysics` _sphere true)
  (`PrimitiveComponent.SetPhysicsLinearVelocity` _sphere (`KismetMathLibrary.MakeVector` 0.0) false "None")
  (`PrimitiveComponent.SetPhysicsAngularVelocityInDegrees` _sphere (`KismetMathLibrary.MakeVector` 0.0) false "None"))

(fn `UserConstructionScript`)