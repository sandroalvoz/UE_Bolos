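; Bowling lane actor that runs a solo ten-pin game, spawning a triangle of pins and a ball if needed.
; Tick detects a released ball stopping downlane or falling, then after a delay EvaluateRoll counts knocked pins and removes or resets them.
; Scores are recomputed from the roll history with strike, spare and tenth-frame rules.
; Three text displays show partly Spanish status and totals, and a new game starts automatically after game over.
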(event `self.ReceiveBeginPlay`
  (`self.SpawnPins`)
  (`/Engine/EditorBlueprintResources/StandardMacros.IsValid` (`self.Ball`)
    (:`Is Valid`
      (`self.NewGame`))
    (:`Is Not Valid`
      (bind _returnvalue (`|SpawnActorFromClass` "/Game/Blueprints/BowlingBall.BowlingBall_C" (`SceneComponent.K2_GetComponentToWorld` (`self.BallSpawn`)) "AlwaysSpawn" "MultiplyWithRoot" null null))
      (set `self.Ball` _returnvalue)
      (`self.NewGame`))))

(event `self.ReceiveTick`
  (params (DeltaSeconds :type "Float (single-precision)"))
  (bind _ball (`self.Ball`))
  (bind _sphere (`/Game/Blueprints/BowlingBall.Sphere` _ball))
  (bind _returnvalue (`KismetMathLibrary.InverseTransformLocation` (`self.GetTransform`) (`SceneComponent.K2_GetComponentLocation` _sphere)))
  (if (not (`self.bEvaluating`))
    (`/Engine/EditorBlueprintResources/StandardMacros.IsValid` _ball
      (:`Is Valid`
        (bind _returnvalue_2 (`PrimitiveComponent.GetPhysicsLinearVelocity` _sphere "None"))
        (if (and (not (`/Game/Blueprints/BowlingBall.bIsHeld` _ball)) (or (and (> (.x _returnvalue) 150.0) (< (`KismetMathLibrary.VSize` _returnvalue_2) 3.0)) (< (.z _returnvalue) -100.0)))
          (set `self.bEvaluating` true)
          (`KismetSystemLibrary.Delay` 3.0)
          (`self.EvaluateRoll`)
          (if (`self.bGameOver`)
            (`KismetSystemLibrary.Delay` 6.0)
            (`self.NewGame`)
            (set `self.bEvaluating` false)
            (else
              (set `self.bEvaluating` false))))))))

(fn `ComputeScore`
  (returns (Score :type Integer))
  (bind _scoreindex (`self.ScoreIndex`))
  (set `self.ScoreIndex` 0)
  (set `self.ScoreSum` 0)
  (for _ (range 10)
    (bind _pins (`self.RollAt` _scoreindex))
    (bind _pins_2 (`self.RollAt` (+ _scoreindex 1)))
    (bind _pins_3 (`self.RollAt` (+ _scoreindex 2)))
    (if (== _pins 10)
      (set `self.ScoreSum` (+ (`self.ScoreSum`) (+ 10 (+ _pins_2 _pins_3))))
      (set `self.ScoreIndex` (+ _scoreindex 1))
      (elif (== (+ _pins _pins_2) 10)
        (set `self.ScoreSum` (+ (`self.ScoreSum`) (+ 10 _pins_3)))
        (set `self.ScoreIndex` (+ _scoreindex 2))
        (else
          (set `self.ScoreSum` (+ (`self.ScoreSum`) (+ _pins _pins_2)))
          (set `self.ScoreIndex` (+ _scoreindex 2))))))
  (return (`self.ScoreSum`)))

(fn `CountKnockedPins`
  (returns (Count :type Integer))
  (set `self.KnockedCounter` 0)
  (for _array_element (`self.Pins`)
    (bind _bknockeddown (`/Game/Blueprints/Bowling/BP_BowlingPin.IsKnockedDown` _array_element))
    (if _bknockeddown
      (set `self.KnockedCounter` (+ (`self.KnockedCounter`) 1))))
  (return (`self.KnockedCounter`)))

(fn `EvaluateRoll`
  (bind _rollinframe (`self.RollInFrame`))
  (bind _ball (`self.Ball`))
  (bind _count (`self.CountKnockedPins`))
  (bind _returnvalue (- _count (`self.PinsDownBefore`)))
  (`KismetArrayLibrary.Array_Add` (`self.Rolls`) _returnvalue)
  (set `self.LastRollPins` _returnvalue)
  (bind _returnvalue_2 (== _count 10))
  (if (and _returnvalue_2 (`self.bRackFresh`))
    (set `self.ResultMessage` "STRIKE!")
    (elif _returnvalue_2
      (set `self.ResultMessage` "SPARE!")
      (else
        (set `self.ResultMessage` (`KismetStringLibrary.Concat_StrStr` (`KismetStringLibrary.Conv_IntToString` _returnvalue) " bolos")))))
  (if (< (`self.CurrentFrame`) 10)
    (if (or _returnvalue_2 (== _rollinframe 2))
      (`self.NextFrame`)
      (else
        (`self.RemoveKnockedPins`)
        (set `self.PinsDownBefore` _count)
        (set `self.RollInFrame` 2)))
    (else
      (bind _pins (`self.RollAt` (- (`KismetArrayLibrary.Array_Length` (`self.Rolls`)) 2)))
      (if (or (== _rollinframe 1) (and (== _rollinframe 2) (or (== _pins 10) _returnvalue_2)))
        (set `self.RollInFrame` (+ _rollinframe 1))
        (if _returnvalue_2
          (`self.ResetAllPins`)
          (set `self.PinsDownBefore` 0)
          (else
            (`self.RemoveKnockedPins`)
            (set `self.PinsDownBefore` _count)))
        (else
          (set `self.bGameOver` true)))))
  (`/Engine/EditorBlueprintResources/StandardMacros.IsValid` _ball
    (:`Is Valid`
      (`/Game/Blueprints/BowlingBall.ResetBall` _ball)
      (`self.UpdateScoreText`))
    (:`Is Not Valid`
      (`self.UpdateScoreText`))))

(fn `NewGame`
  (`KismetArrayLibrary.Array_Clear` (`self.Rolls`))
  (set `self.CurrentFrame` 1)
  (set `self.RollInFrame` 1)
  (set `self.PinsDownBefore` 0)
  (set `self.LastRollPins` 0)
  (set `self.bGameOver` false)
  (set `self.ResultMessage` "")
  (`self.ResetAllPins`)
  (`self.UpdateScoreText`))

(fn `NextFrame`
  (set `self.CurrentFrame` (+ (`self.CurrentFrame`) 1))
  (set `self.RollInFrame` 1)
  (set `self.PinsDownBefore` 0)
  (`self.ResetAllPins`))

(fn `RemoveKnockedPins`
  (for _array_element (`self.Pins`)
    (bind _bknockeddown (`/Game/Blueprints/Bowling/BP_BowlingPin.IsKnockedDown` _array_element))
    (if _bknockeddown
      (`/Game/Blueprints/Bowling/BP_BowlingPin.RemovePin` _array_element)))
  (set `self.bRackFresh` false))

(fn `ResetAllPins`
  (for _array_element (`self.Pins`)
    (`/Game/Blueprints/Bowling/BP_BowlingPin.ResetPin` _array_element))
  (set `self.bRackFresh` true))

(fn `RollAt`
  (params (Index :type Integer))
  (returns (Pins :type Integer))
  (bind _rolls (`self.Rolls`))
  (if (`KismetArrayLibrary.Array_IsValidIndex` _rolls Index)
    (return (`|GetArrayItem` _rolls Index))
    (else
      (return 0))))

(fn `SpawnPins`
  (for _index (range 4)
    (for _index_2 (range (+ (- (+ _index 1) 1) 1))
      (bind _returnvalue (`KismetMathLibrary.Conv_IntToDouble` _index))
      (bind _returnvalue_2 (`|SpawnActorFromClass` "/Game/Blueprints/Bowling/BP_BowlingPin.BP_BowlingPin_C" (`KismetMathLibrary.MakeTransform` (`KismetMathLibrary.TransformLocation` (`self.GetTransform`) (`KismetMathLibrary.MakeVector` (+ 1050.0 (* _returnvalue 26.4)) (* (- (`KismetMathLibrary.Conv_IntToDouble` _index_2) (* _returnvalue 0.5)) 30.48) 22.3)) (`self.K2_GetActorRotation`)) "AlwaysSpawn" "MultiplyWithRoot" null null))
      (`KismetArrayLibrary.Array_Add` (`self.Pins`) _returnvalue_2))))

(fn `UpdateScoreText`
  (bind _returnvalue (`KismetStringLibrary.Concat_StrStr` (`KismetMathLibrary.SelectString` "Fin de la partida" (`KismetStringLibrary.Concat_StrStr` (`KismetStringLibrary.Concat_StrStr` "Frame " (`KismetStringLibrary.Conv_IntToString` (`self.CurrentFrame`))) (`KismetStringLibrary.Concat_StrStr` " - Tirada " (`KismetStringLibrary.Conv_IntToString` (`self.RollInFrame`)))) (`self.bGameOver`)) (`KismetStringLibrary.Concat_StrStr` "   " (`self.ResultMessage`))))
  (bind _score (`self.ComputeScore`))
  (set `self.TotalScore` _score)
  (bind _returnvalue_2 (`KismetStringLibrary.Concat_StrStr` "Total: " (`KismetStringLibrary.Conv_IntToString` _score)))
  (`TextRenderComponent.K2_SetText` (`self.ScoreText`) (`KismetTextLibrary.Conv_StringToText` _returnvalue_2))
  (`TextRenderComponent.K2_SetText` (`self.InfoText`) (`KismetTextLibrary.Conv_StringToText` _returnvalue))
  (`TextRenderComponent.K2_SetText` (`self.NearText`) (`KismetTextLibrary.Conv_StringToText` (`KismetStringLibrary.Concat_StrStr` _returnvalue (`KismetStringLibrary.Concat_StrStr` "   " _returnvalue_2)))))

(fn `UserConstructionScript`)