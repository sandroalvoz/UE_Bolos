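; BP_BowlingPin is a physics-simulated bowling pin that reports whether it has fallen and can be removed or reset.
; It stores its spawn transform on BeginPlay, and IsKnockedDown compares tilt via the up vector and drop below start height, or counts removed pins as down.
; RemovePin hides it and disables physics and collision, while ResetPin teleports it back, restores visibility and collision, and zeroes velocities.
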(event `self.ReceiveBeginPlay`
  (set `self.StartTransform` (`self.GetTransform`)))

(fn `IsKnockedDown`
  (returns (bKnockedDown :type Boolean))
  (return (or (`self.bIsRemoved`) (or (< (.z (`self.GetActorUpVector`)) 0.8) (< (.z (`self.K2_GetActorLocation`)) (- (.z (.location (`self.StartTransform`))) 10.0))))))

(fn `RemovePin`
  (`PrimitiveComponent.SetSimulatePhysics` (`self.StaticMeshComponent`) false)
  (`self.SetActorHiddenInGame` true)
  (`self.SetActorEnableCollision` false)
  (set `self.bIsRemoved` true))

(fn `ResetPin`
  (bind _staticmeshcomponent (`self.StaticMeshComponent`))
  (`PrimitiveComponent.SetSimulatePhysics` _staticmeshcomponent false)
  (`self.K2_SetActorTransform` (`self.StartTransform`) false true)
  (`self.SetActorHiddenInGame` false)
  (`self.SetActorEnableCollision` true)
  (set `self.bIsRemoved` false)
  (`PrimitiveComponent.SetSimulatePhysics` _staticmeshcomponent true)
  (`PrimitiveComponent.SetPhysicsLinearVelocity` _staticmeshcomponent (`KismetMathLibrary.MakeVector` 0.0) false "None")
  (`PrimitiveComponent.SetPhysicsAngularVelocityInDegrees` _staticmeshcomponent (`KismetMathLibrary.MakeVector` 0.0) false "None"))

(fn `UserConstructionScript`)